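; BP_Snow is a snowfall effect actor that varies its wind over time and can be switched off indoors.
; From BeginPlay, ChangeWind repeatedly sets a random wind power on the Snow particle component and a random yaw on the actor, re-calling itself after a random delay.
; IsInside and IsOutside events set the spawn rate parameter to stop or restore the snow; their callers are not in this file.
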(event `self.ReceiveBeginPlay`
  (`self.ChangeWind`))

(event `ChangeWind`
  (`NiagaraComponent.SetVariableFloat` (`self.Snow`) "User.WindPower" (`KismetMathLibrary.RandomFloatInRange` -1000.0 1000.0))
  (`self.K2_SetActorRotation` (`KismetMathLibrary.MakeRotator` 0.0 0.0 (`KismetMathLibrary.RandomFloatInRange` 0.0 360.0)))
  (`KismetSystemLibrary.PrintString` "Changing Wind" false)
  (`KismetSystemLibrary.Delay` (`KismetMathLibrary.RandomFloatInRange` 5.0 20.0))
  (`self.ChangeWind`))

(event `/Game/BPI_SnowChange.IsInside`
  (`NiagaraComponent.SetVariableFloat` (`self.Snow`) "User.SnowRate" 0.0))

(event `/Game/BPI_SnowChange.IsOutside`
  (`NiagaraComponent.SetVariableFloat` (`self.Snow`) "User.SnowRate" 2000.0))

(fn `UserConstructionScript`)