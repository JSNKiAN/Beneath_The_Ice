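; Scene capture actor for snow deformation that follows the player and maintains a persistent render target of the captured area.
; Each tick it moves in XY on a pixel-sized world grid to avoid sub-texel drift, publishing its location and capture size to MPC_Capture.
; It then draws M_DrawToPersistant into RT_Persistant with the normalized move offset, so accumulated data stays world-aligned as the capture scrolls.
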(event `self.ReceiveBeginPlay`
  (`KismetMaterialLibrary.SetScalarParameterValue` "/Game/SnowDeform/Material/MPC_Capture.MPC_Capture" "CaptureSize" (`SceneCaptureComponent2D.OrthoWidth` (`self.SceneCaptureComponent2D`)))
  (bind _returnvalue (`KismetMaterialLibrary.CreateDynamicMaterialInstance` "/Game/SnowDeform/Material/M_DrawToPersistant.M_DrawToPersistant"))
  (set `self.DrawMaterial` _returnvalue)
  (`KismetRenderingLibrary.ClearRenderTarget2D` "/Game/SnowDeform/Textures/RT_Capture.RT_Capture")
  (`KismetRenderingLibrary.ClearRenderTarget2D` "/Game/SnowDeform/Textures/RT_Persistant.RT_Persistant"))

(event `self.ReceiveTick`
  (params (DeltaSeconds :type "Float (single-precision)"))
  (`self.MoveCapture`)
  (`self.DrawToPersistant`))

(fn `DrawToPersistant`
  (bind (_returnvalue_x _returnvalue_y) (`KismetMathLibrary.BreakVector2D` (/ (`self.MoveOffset`) (`SceneCaptureComponent2D.OrthoWidth` (`self.SceneCaptureComponent2D`)))))
  (`MaterialInstanceDynamic.SetVectorParameterValue` (`self.DrawMaterial`) "Offset" (make `LinearColor` _returnvalue_x _returnvalue_y 0.0 1.0))
  (`KismetRenderingLibrary.DrawMaterialToRenderTarget` "/Game/SnowDeform/Textures/RT_Persistant.RT_Persistant" (`self.DrawMaterial`)))

(fn `MoveCapture`
  (bind (_returnvalue_x _returnvalue_y) (`KismetMathLibrary.BreakVector` (`self.K2_GetActorLocation` (`GameplayStatics.GetPlayerCharacter` 0))))
  (bind (_returnvalue_x_2 _returnvalue_y_2) (`KismetMathLibrary.BreakVector` (- (`self.SnaptoPixelWorldSize` _returnvalue_x _returnvalue_y (* (`SceneCaptureComponent2D.OrthoWidth` (`self.SceneCaptureComponent2D`)) (/ 1.0 512.0))) (`self.K2_GetActorLocation`))))
  (bind _output_get (set `self.MoveOffset` (`KismetMathLibrary.MakeVector2D` _returnvalue_x_2 _returnvalue_y_2)))
  (`self.K2_AddActorWorldOffset` (`KismetMathLibrary.MakeVector` (`KismetMathLibrary.BreakVector2D` _output_get) (`.Y` (`KismetMathLibrary.BreakVector2D` _output_get))))
  (`KismetMaterialLibrary.SetVectorParameterValue` "/Game/SnowDeform/Material/MPC_Capture.MPC_Capture" "CaptureLocation" (`KismetMathLibrary.Conv_VectorToLinearColor` (`self.K2_GetActorLocation`))))

(fn `UserConstructionScript`)