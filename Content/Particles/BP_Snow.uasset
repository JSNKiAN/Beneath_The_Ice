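; Snow weather actor that drives a particle component named Snow with shifting wind and switchable intensity levels.
; From BeginPlay, ChangeWind randomizes the wind power parameter and the actor's yaw, then calls itself again after a random delay.
; IndoorSnow, NormalSnow and HeavySnow events set the spawn rate through User parameters; normal and heavy also set sprite size, while indoor changes only the rate.
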(event `self.ReceiveBeginPlay`
  (`self.ChangeWind`))

(event `ChangeWind`
  (`NiagaraComponent.SetVariableFloat` (`self.Snow`) "User.WindPower" (`KismetMathLibrary.RandomFloatInRange` -1000.0 1000.0))
  (`self.K2_SetActorRotation` (`KismetMathLibrary.MakeRotator` 0.0 0.0 (`KismetMathLibrary.RandomFloatInRange` 0.0 360.0)))
  (`KismetSystemLibrary.PrintString` "Changing Wind" false)
  (`KismetSystemLibrary.Delay` (`KismetMathLibrary.RandomFloatInRange` 5.0 20.0))
  (`self.ChangeWind`))

(event `/Game/Particles/BPI_SnowChange.IndoorSnow`
  (`NiagaraComponent.SetVariableFloat` (`self.Snow`) "User.SnowRate" 100.0))

(event `/Game/Particles/BPI_SnowChange.NormalSnow`
  (bind _snow (`self.Snow`))
  (`NiagaraComponent.SetVariableFloat` _snow "User.SnowRate" 2000.0)
  (`NiagaraComponent.SetVariableFloat` _snow "User.SpriteSizeMin" 1.0)
  (`NiagaraComponent.SetVariableFloat` _snow "User.SpriteSizeMax" 5.0))

(event `/Game/Particles/BPI_SnowChange.HeavySnow`
  (bind _snow (`self.Snow`))
  (`NiagaraComponent.SetVariableFloat` _snow "User.SnowRate" 5000.0)
  (`NiagaraComponent.SetVariableFloat` _snow "User.SpriteSizeMin" 5.0)
  (`NiagaraComponent.SetVariableFloat` _snow "User.SpriteSizeMax" 10.0))

(fn `UserConstructionScript`)