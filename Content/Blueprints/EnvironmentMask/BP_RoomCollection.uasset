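; Room volume actor that groups objects implementing BPI_TransparencySettings so they can be faded as one room.
; GatherActors rebuilds StaticObjects with a near-zero-length multi box trace on Visibility matching the Box component, with debug drawing on.
; FadeRoom sends fade-in or fade-out interface messages to everything in StaticObjects and DynamicObjects.
; DynamicObjects is not populated here, and neither event is called within this Blueprint.
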(event `GatherActors`
  (bind _box (`self.Box`))
  (bind _returnvalue (`SceneComponent.K2_GetComponentLocation` _box))
  ;[0.05098 0.05098 0.05098] Clear array for new set
  (`KismetArrayLibrary.Array_Clear` (`self.StaticObjects`))
  (bind _outhits (`KismetSystemLibrary.BoxTraceMulti` :`Start` _returnvalue :`End` (+ _returnvalue (0.0 0.0 0.01)) :`HalfSize` (`BoxComponent.GetScaledBoxExtent` _box) :`Orientation` (`SceneComponent.K2_GetComponentRotation` _box) :`TraceChannel` "TraceTypeQuery1" :`DrawDebugType` "ForDuration"))
  (for _array_element _outhits
    (bind (_bblockinghit _binitialoverlap _time _distance _location _impactpoint _normal _impactnormal _physmat _hitactor) (`GameplayStatics.BreakHitResult` _array_element))
    (if (`KismetSystemLibrary.DoesImplementInterface` _hitactor "/Game/Blueprints/EnvironmentMask/BPI_TransparencySettings.BPI_TransparencySettings_C")
      (`KismetArrayLibrary.Array_Add` (`self.StaticObjects`) _hitactor))))

(event `FadeRoom`
  (params (bShouldFade :type Boolean))
  (for _array_element (`self.StaticObjects`)
    (if bShouldFade
      (message `/Game/Blueprints/EnvironmentMask/BPI_TransparencySettings.FadeIn` _array_element)
      (else
        (message `/Game/Blueprints/EnvironmentMask/BPI_TransparencySettings.FadeOut` _array_element))))
  (for _array_element_2 (`self.DynamicObjects`)
    (if bShouldFade
      (message `/Game/Blueprints/EnvironmentMask/BPI_TransparencySettings.FadeIn` _array_element_2)
      (else
        (message `/Game/Blueprints/EnvironmentMask/BPI_TransparencySettings.FadeOut` _array_element_2)))))

(fn `UserConstructionScript`)