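; Environment mesh actor that can fade out and back in, toggling whether it blocks the Visibility trace channel.
; BeginPlay creates a dynamic material instance from the mesh's first material slot.
; FadeOut and Fadein play and reverse the Fader timeline, whose update sets FadeAmount, though the value shown is a constant zero.
; IsFaded returns the Faded flag, which no graph here sets.
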(event `self.ReceiveBeginPlay`
  (bind _staticmesh (`self.StaticMesh`))
  (bind _returnvalue (`PrimitiveComponent.CreateDynamicMaterialInstance` _staticmesh 0 (`PrimitiveComponent.GetMaterial` _staticmesh 0) "None"))
  (set `self.MI` _returnvalue))

(event `/Game/Blueprints/EnvironmentMask/BPI_TransparencySettings.FadeOut`
  (`PrimitiveComponent.SetCollisionResponseToChannel` (`self.StaticMesh`) "ECC_Visibility" "ECR_Ignore")
  (`Timeline|Fader` :!label _label
    (:`Update`
      (`MaterialInstanceDynamic.SetScalarParameterValue` (`self.MI`) "FadeAmount" 0.0))))

(event `/Game/Blueprints/EnvironmentMask/BPI_TransparencySettings.FadeIn`
  (`PrimitiveComponent.SetCollisionResponseToChannel` (`self.StaticMesh`) "ECC_Visibility" "ECR_Block")
  (goto _label :!via `Reverse`))

(fn `IsFaded`
  (returns (bIsFaded :type Boolean))
  (return (`self.bFaded`)))

(fn `UserConstructionScript`)