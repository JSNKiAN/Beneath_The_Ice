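; BP_StairMovement is a trigger actor, named for stairs, that slows the player's walking while they are inside its Box volume.
; On BeginPlay it casts the first player pawn to BP_Player and caches the reference.
; The Box overlap events compare the overlapping actor to that reference, lowering the CharacterMovement MaxWalkSpeed on entry and setting a hardcoded normal speed on exit rather than restoring the previous value.
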(event `self.ReceiveBeginPlay`
  ;[0.05098 0.05098 0.05098] Get Player Actor
  (bind _asbp_player (cast `/Game/Blueprints/BP_Player` (`GameplayStatics.GetPlayerPawn` 0)))
  (set `self.As BP Player` _asbp_player))

(event `self.Box.OnComponentBeginOverlap`
  (params (OverlappedComponent :type "PrimitiveComponent Object Reference") (OtherActor :type "Actor Object Reference") (OtherComp :type "PrimitiveComponent Object Reference") (OtherBodyIndex :type Integer) (bFromSweep :type Boolean) (SweepResult :type "HitResult Structure (by ref)"))
  ;[0.05098 0.05098 0.05098] Check if Player Actor overlap
  (if (== OtherActor (`self.As BP Player`))
    (set `CharacterMovementComponent.MaxWalkSpeed` 100.0 (`Character.CharacterMovement` (`self.As BP Player`)))))

(event `self.Box.OnComponentEndOverlap`
  (params (OverlappedComponent :type "PrimitiveComponent Object Reference") (OtherActor :type "Actor Object Reference") (OtherComp :type "PrimitiveComponent Object Reference") (OtherBodyIndex :type Integer))
  ;[0.05098 0.05098 0.05098] Check if Player Actor overlap
  (if (== OtherActor (`self.As BP Player`))
    (set `CharacterMovementComponent.MaxWalkSpeed` 200.0 (`Character.CharacterMovement` (`self.As BP Player`)))))

(fn `UserConstructionScript`)