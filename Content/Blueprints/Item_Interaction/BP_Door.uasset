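; BP_Door is an interactable door that toggles open and closed by swinging its static mesh.
; BeginPlay stores the starting rotation, and a Timeline lerps yaw to 90 degrees below it, playing from start to open and reversing to close.
; Interact is gated by CanPressE and CanInteract, which is cleared on use and restored by a short Delay wired to the Timeline's Update rather than Finished.
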(event `self.ReceiveBeginPlay`
  (set `self.Starting Rotation` (`SceneComponent.RelativeRotation` (`self.StaticMesh`))))

(event `/Game/Blueprints/Item_Interaction/BPI_Interaction.Interact`
  (bind (_starting_rotation_roll _starting_rotation_pitch _starting_rotation_yaw) (`KismetMathLibrary.BreakRotator` (`self.Starting Rotation`)))
  (if (`self.CanPressE`)
    (if (`self.CanInteract`)
      (set `self.CanInteract` false)
      (if (`self.Opened`)
        (set `self.Opened` false)
        (bind (_direction _alpha) (`Timeline|Timeline` :!via `Reverse` :!label _label)
          (:`Update`
            (`SceneComponent.K2_SetRelativeRotation` (`self.StaticMesh`) (`KismetMathLibrary.MakeRotator` _starting_rotation_roll _starting_rotation_pitch (`KismetMathLibrary.Lerp` _starting_rotation_yaw (- _starting_rotation_yaw 90.0) _alpha)) false false)
            (`KismetSystemLibrary.Delay` 0.2)
            (set `self.CanInteract` true)))
        (else
          (set `self.Opened` true)
          (goto _label :!via `PlayFromStart`))))))

(fn `UserConstructionScript`
  (`parent.UserConstructionScript`))