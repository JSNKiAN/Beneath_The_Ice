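; Master interactable item that combines highlight prompts, key unlocking, dialogue and collecting.
; Sphere overlap shows a semi-highlight and prompt widget for BP_Player, and trace events animate the prompt and switch highlights.
; Interact, optionally one-time, messages an unlock actor, plays dialogue lines timed by text length, and hides collectibles.
; FloatingDialogue fires that same sequence once on any sphere overlap, bypassing the CanInteract check.
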(event `/Game/Blueprints/Item_Interaction/BPI_Interaction.Interact`
  (bind _staticmesh (`self.StaticMesh`))
  (if (`self.CanInteract?`)
    (if (`self.InteractOnlyOnce?`)
      ;[0.05098 0.05098 0.05098] One Time Interact
      (set `self.CanInteract?` false)
      (set `self.Interaction Widget` null)
      (`SceneComponent.SetVisibility` (`self.WidgetPrompt`) false false)
      (`MeshComponent.SetOverlayMaterial` (`self.StaticMesh`) null))
    (`|ExecutionSequence` :!label _label
      (:`then_0`
        ;[0.05098 0.05098 0.05098] Key System
        (bind _returnvalue (`GameplayStatics.GetActorOfClass` (`self.ActorUnlock`)))
        (message `/Game/Blueprints/Item_Interaction/BPI_Interaction.UnlockInteract` _returnvalue))
      (:`then_1`
        ;[0.05098 0.05098 0.05098] Dialogue System
        (if (`self.Dialogue?`)
          (`/Engine/EditorBlueprintResources/StandardMacros.DoOnce` false :!label _label_2
            (:`Completed`
              (`/Engine/EditorBlueprintResources/StandardMacros.IncrementInt` (`self.talkIndex`) :!label _label_3
                (:`  `
                  ;;[0.05098 0.05098 0.05098] Stop once Index reached Dialogue length
                  (if (< (`self.talkIndex`) (`KismetArrayLibrary.Array_Length` (`self.Dialogue`)))
                    (`self.Dialogue Widget`
                      (:`then`
                        _)
                      (:`else`
                        (bind _returnvalue_2 (`|CreateWidget` "/Game/Blueprints/Item_Interaction/WBP_Dialogue.WBP_Dialogue_C" (`GameplayStatics.GetPlayerController` 0)))
                        (bind _output_get (set `self.Dialogue Widget` _returnvalue_2))
                        (`UserWidget.AddToViewport` _output_get 0)))
                    (`TextBlock.SetText` (`/Game/Blueprints/Item_Interaction/WBP_Dialogue.TalkText` (`self.Dialogue Widget`)) (`KismetTextLibrary.Conv_StringToText` (`|GetArrayItem` (`self.Dialogue`) (`self.talkIndex`))))
                    (`TextBlock.SetText` (`/Game/Blueprints/Item_Interaction/WBP_Dialogue.NameText` (`self.Dialogue Widget`)) (`KismetTextLibrary.Conv_StringToText` (`|GetArrayItem` (`self.Name`) (`self.talkIndex`))))
                    (`Image.SetBrushFromTexture` (`/Game/Blueprints/Item_Interaction/WBP_Dialogue.PortraitImage` (`self.Dialogue Widget`)) (`|GetArrayItem` (`self.Portrait`) (`self.talkIndex`)) true)
                    (`KismetSystemLibrary.Delay` (/ (`KismetStringLibrary.Len` (`|GetArrayItem` (`self.Dialogue`) (`self.talkIndex`))) (`self.TalkSpeed`)))
                    (goto _label_3)
                    (else
                      (`Widget.RemoveFromParent` (`self.Dialogue Widget`))
                      (set `self.Dialogue Widget` null)
                      (set `self.talkIndex` -1)
                      (goto _label_2 :!via `Reset`)))))))))
      (:`then_2`
        ;[0.05098 0.05098 0.05098] Collect System
        (if (`self.Collect?`)
          (`SceneComponent.SetVisibility` _staticmesh false false)
          (`PrimitiveComponent.SetCollisionEnabled` _staticmesh "NoCollision"))))))

(event `OverlapEvent`
  ;[0.05098 0.05098 0.05098] Volume Trigger System
  (`/Engine/EditorBlueprintResources/StandardMacros.DoOnce` false
    (:`Completed`
      (goto _label))))

(event `self.ReceiveBeginPlay`)

(event `self.Sphere.OnComponentBeginOverlap`
  (params (OverlappedComponent :type "PrimitiveComponent Object Reference") (OtherActor :type "Actor Object Reference") (OtherComp :type "PrimitiveComponent Object Reference") (OtherBodyIndex :type Integer) (bFromSweep :type Boolean) (SweepResult :type "HitResult Structure (by ref)"))
  (bind _widgetprompt (`self.WidgetPrompt`))
  (if (`self.FloatingDialogue`)
    (`self.OverlapEvent`))
  (cast `/Game/Blueprints/BP_Player` OtherActor)
  (if (`self.CanInteract?`)
    (set `self.CanClickOn` true)
    (`MeshComponent.SetOverlayMaterial` (`self.StaticMesh`) "/Game/Material/M_Highlight_Semi.M_Highlight_Semi")
    (bind _returnvalue (`|CreateWidget` "/Game/Blueprints/Item_Interaction/W_UI_Interact.W_UI_Interact_C" null "ActionName"))
    (bind _output_get (set `self.Interaction Widget` _returnvalue))
    (`WidgetComponent.SetWidget` _widgetprompt _output_get)
    (`SceneComponent.SetVisibility` _widgetprompt true false)
    ;[0.05098 0.05098 0.05098] Sets Action Name
    (`/Game/Blueprints/Item_Interaction/W_UI_Interact.SetDesiredActionName` (`self.Interaction Widget`) (`self.ActionName`))))

(event `self.Sphere.OnComponentEndOverlap`
  (params (OverlappedComponent :type "PrimitiveComponent Object Reference") (OtherActor :type "Actor Object Reference") (OtherComp :type "PrimitiveComponent Object Reference") (OtherBodyIndex :type Integer))
  (cast `/Game/Blueprints/BP_Player` OtherActor)
  (set `self.CanClickOn` false)
  (`MeshComponent.SetOverlayMaterial` (`self.StaticMesh`) null)
  (set `self.Interaction Widget` null)
  (`SceneComponent.SetVisibility` (`self.WidgetPrompt`) false false))

(event `/Game/Blueprints/Item_Interaction/BPI_Interaction.Can Receive Trace`
  (params (`Can Interact` :type Boolean))
  (if (`self.CanInteract?`)
    (if `Can Interact`
      (bind _interaction_widget (`self.Interaction Widget`)
        (:`then`
          (if (not (`self.HintVisible`))
            (`UserWidget.PlayAnimation` _interaction_widget (`/Game/Blueprints/Item_Interaction/W_UI_Interact.PopUp` _interaction_widget) 0.0 1 "Forward" 1.5 false)
            (set `self.HintVisible` true)
            (set `self.CanClickOn` true)
            (`MeshComponent.SetOverlayMaterial` (`self.StaticMesh`) "/Game/Material/M_Highlight.M_Highlight")))
        (:`else`))
      (else
        (bind _interaction_widget_2 (`self.Interaction Widget`)
          (:`then`
            (if (`self.HintVisible`)
              (`UserWidget.PlayAnimation` _interaction_widget_2 (`/Game/Blueprints/Item_Interaction/W_UI_Interact.PopUp` _interaction_widget_2) 0.0 1 "Reverse" 1.5 false)
              (set `self.HintVisible` false)
              (set `self.CanClickOn` false)
              (`MeshComponent.SetOverlayMaterial` (`self.StaticMesh`) "/Game/Material/M_Highlight_Semi.M_Highlight_Semi")))
          (:`else`))))))

(fn `UserConstructionScript`)