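; BP_NPC is an interactable NPC that plays a self-advancing dialogue when its Interact event fires.
; It creates a WBP_Dialogue widget and steps through its dialogue and name arrays, showing each line for a time based on text length and talk speed.
; A DoOnce blocks re-triggering during playback, then resets once the last line ends, the widget is removed and the index is cleared.
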(event `/Game/Blueprints/Item_Interaction/BPI_Interaction.Interact`
  (`/Engine/EditorBlueprintResources/StandardMacros.DoOnce` false :!label _label
    (:`Completed`
      (`/Engine/EditorBlueprintResources/StandardMacros.IncrementInt` (`self.talkIndex_0`) :!label _label_2
        (:`  `
          ;[0.05098 0.05098 0.05098] Stop once Index reached Dialogue length
          (if (< (`self.talkIndex_0`) (`KismetArrayLibrary.Array_Length` (`self.Dialogue_0`)))
            (`self.Dialogue Widget_0`
              (:`then`
                _)
              (:`else`
                (bind _returnvalue (`|CreateWidget` "/Game/Blueprints/Item_Interaction/WBP_Dialogue.WBP_Dialogue_C" (`GameplayStatics.GetPlayerController` 0)))
                (bind _output_get (set `self.Dialogue Widget_0` _returnvalue))
                (`UserWidget.AddToViewport` _output_get 0)))
            (`TextBlock.SetText` (`/Game/Blueprints/Item_Interaction/WBP_Dialogue.TalkText` (`self.Dialogue Widget_0`)) (`KismetTextLibrary.Conv_StringToText` (`|GetArrayItem` (`self.Dialogue_0`) (`self.talkIndex_0`))))
            (`TextBlock.SetText` (`/Game/Blueprints/Item_Interaction/WBP_Dialogue.NameText` (`self.Dialogue Widget_0`)) (`KismetTextLibrary.Conv_StringToText` (`|GetArrayItem` (`self.Name_0`) (`self.talkIndex_0`))))
            (`KismetSystemLibrary.Delay` (/ (`KismetStringLibrary.Len` (`|GetArrayItem` (`self.Dialogue_0`) (`self.talkIndex_0`))) (`self.TalkSpeed_0`)))
            (goto _label_2)
            (else
              (`Widget.RemoveFromParent` (`self.Dialogue Widget_0`))
              (set `self.Dialogue Widget_0` null)
              (set `self.talkIndex_0` -1)
              (goto _label :!via `Reset`))))))))

(fn `UserConstructionScript`
  (`parent.UserConstructionScript`))