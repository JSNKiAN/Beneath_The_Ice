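; BP_OutDoor is an interactable door that swings open and closed with matching sounds.
; Interact, gated by CanClickOn and CanInteract, toggles Opened and plays or reverses a Timeline that lerps the mesh yaw 90 degrees from its BeginPlay rotation.
; CanInteract blocks repeat input until a short Delay on the Timeline update restores it, or UnlockInteract sets it.
; Both sounds play at world origin rather than at the door.
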(event `/Game/Blueprints/Item_Interaction/BPI_Interaction.UnlockInteract`
  (set `self.CanInteract?` true))

(event `self.ReceiveBeginPlay`
  (set `self.Starting Rotation` (`SceneComponent.RelativeRotation` (`self.StaticMesh`))))

(event `self.Interact`
  (bind (_starting_rotation_roll _starting_rotation_pitch _starting_rotation_yaw) (`KismetMathLibrary.BreakRotator` (`self.Starting Rotation`)))
  (if (`self.CanClickOn`)
    (if (`self.CanInteract?`)
      (set `self.CanInteract?` false)
      (if (`self.Opened`)
        (set `self.Opened` false)
        (`GameplayStatics.PlaySoundAtLocation` "/Game/Sounds/Door/Door-Closed.Door-Closed" (0.0 0.0 0.0) (struct) 1.0 1.0 0.0 null null null null)
        (bind (_direction _alpha) (`Timeline|Timeline` :!via `Reverse` :!label _label)
          (:`Update`
            (`SceneComponent.K2_SetRelativeRotation` (`self.StaticMesh`) (`KismetMathLibrary.MakeRotator` _starting_rotation_roll _starting_rotation_pitch (`KismetMathLibrary.Lerp` _starting_rotation_yaw (- _starting_rotation_yaw 90.0) _alpha)) false false)
            (`KismetSystemLibrary.Delay` 0.2)
            (set `self.CanInteract?` true)))
        (else
          (set `self.Opened` true)
          (`GameplayStatics.PlaySoundAtLocation` "/Game/Sounds/Door/Door-Open.Door-Open" (0.0 0.0 0.0) (struct) 1.0 1.0 0.0 null null null null)
          (goto _label :!via `PlayFromStart`))))))

(fn `UserConstructionScript`
  (`parent.UserConstructionScript`))