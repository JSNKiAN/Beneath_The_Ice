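; Player controller that makes the BP_Player character look at the mouse cursor.
; BeginPlay shows the cursor and seeds the look-at location from the cursor's Visibility hit.
; Each tick, it smooths that location toward the current hit with VInterpTo and sends it to the player mesh's anim instance through LookAtMouseMessage.
; An unconnected deprojection line trace is left in the graph, unused.
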(event `self.ReceiveTick`
  (params (DeltaSeconds :type "Float (single-precision)"))
  (`|ExecutionSequence`
    (:`then_0`
      (set `self.Delta Seconds` DeltaSeconds))
    (:`then_1`
      (bind _asbp_player (cast `/Game/Blueprints/BP_Player` (`GameplayStatics.GetPlayerPawn` 0)))
      (bind _output_get (set `self.MouseLoc` (`KismetMathLibrary.VInterpTo` (`self.MouseLoc`) (`.Location` (`GameplayStatics.BreakHitResult` (`self.GetHitResultUnderCursorByChannel` "TraceTypeQuery1"))) (`self.Delta Seconds`) (`self.Look At Speed`))))
      (message `/Game/Blueprints/BPI_Character.LookAtMouse` (`SkeletalMeshComponent.GetAnimInstance` (`Character.Mesh` _asbp_player)) _output_get))))

(event `self.ReceiveBeginPlay`
  (set `self.bShowMouseCursor` true)
  (set `self.MouseLoc` (`.Location` (`GameplayStatics.BreakHitResult` (`self.GetHitResultUnderCursorByChannel` "TraceTypeQuery1")))))

(fn `UserConstructionScript`)