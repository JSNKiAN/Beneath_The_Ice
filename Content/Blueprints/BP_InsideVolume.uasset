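; BP_InsideVolume is a box volume that zooms the player camera in and grows an occlusion mask while something is inside it.
; Box overlap events toggle an Inside flag without filtering which actor triggered them.
; Each tick interpolates mask size and FOV toward inside values, or back to zero and the FOV captured at BeginPlay.
; The results drive a Material Parameter Collection scalar and BP_Player's FollowCamera.
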(event `self.ReceiveBeginPlay`
  ;[0.05098 0.05098 0.05098] Get Player Camera (FOV)
  (bind _asbp_player (cast `/Game/Blueprints/BP_Player` (`GameplayStatics.GetPlayerPawn` 0)))
  (set `self.OriginalFOV` (`CameraComponent.FieldOfView` (`/Game/Blueprints/BP_Player.FollowCamera` _asbp_player))))

(event `self.ReceiveTick`
  (params (DeltaSeconds :type "Float (single-precision)"))
  (`|ExecutionSequence`
    (:`then_0`
      (set `self.Delta Seconds` DeltaSeconds))
    (:`then_1`
      (if (`self.Inside`)
        ;[0.05098 0.05098 0.05098] FInterp Occlusion Mask Size
        (set `self.CurrentOcclusionSize` (`KismetMathLibrary.FInterpTo` (`self.CurrentOcclusionSize`) (`self.OcclusionSize`) (`self.Delta Seconds`) (`self.SizeSpeed`)))
        ;[0.05098 0.05098 0.05098] FInterp Camera Zoom
        (set `self.CurrentFOV` (`KismetMathLibrary.FInterpTo` (`self.CurrentFOV`) 7.0 (`self.Delta Seconds`) (`self.ZoomSpeed`)))
        (else
          (set `self.CurrentOcclusionSize` (`KismetMathLibrary.FInterpTo` (`self.CurrentOcclusionSize`) 0.0 (`self.Delta Seconds`) (`self.SizeSpeed`)))
          (set `self.CurrentFOV` (`KismetMathLibrary.FInterpTo` (`self.CurrentFOV`) (`self.OriginalFOV`) (`self.Delta Seconds`) (`self.ZoomSpeed`))))))
    (:`then_2`
      ;[0.05098 0.05098 0.05098] Update Occlusion Mask Size
      (`KismetMaterialLibrary.SetScalarParameterValue` "/Game/Blueprints/EnvironmentMask/MPC_ParameterCollection.MPC_ParameterCollection" "OcclusionSize" (`self.CurrentOcclusionSize`)))
    (:`then_3`
      ;[0.05098 0.05098 0.05098] Update Player Camera FOV
      (bind _asbp_player (cast `/Game/Blueprints/BP_Player` (`GameplayStatics.GetPlayerPawn` 0)))
      (`CameraComponent.SetFieldOfView` (`/Game/Blueprints/BP_Player.FollowCamera` _asbp_player) (`self.CurrentFOV`)))))

(event `self.Box.OnComponentBeginOverlap`
  (params (OverlappedComponent :type "PrimitiveComponent Object Reference") (OtherActor :type "Actor Object Reference") (OtherComp :type "PrimitiveComponent Object Reference") (OtherBodyIndex :type Integer) (bFromSweep :type Boolean) (SweepResult :type "HitResult Structure (by ref)"))
  (set `self.Inside` true))

(event `self.Box.OnComponentEndOverlap`
  (params (OverlappedComponent :type "PrimitiveComponent Object Reference") (OtherActor :type "Actor Object Reference") (OtherComp :type "PrimitiveComponent Object Reference") (OtherBodyIndex :type Integer))
  (set `self.Inside` false))

(fn `UserConstructionScript`)